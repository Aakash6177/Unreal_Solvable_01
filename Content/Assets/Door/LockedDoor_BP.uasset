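; Locked door Blueprint that the player opens and closes with the interact input while carrying a key.
; Box overlap by the ThirdPersonCharacter caches the character and toggles input and a gate.
; With HasKey, interact passes the gate into a FlipFlop that plays or reverses a timeline lerping door yaw between closed and open angles.
; Without the key, interact bypasses the gate and plays a sound at the door.
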(event OnComponentBeginOverlap(Box)
  (params (OverlappedComponent :type Primitive%20Component%20Object%20Reference) (OtherActor :type Actor%20Object%20Reference) (OtherComp :type Primitive%20Component%20Object%20Reference) (OtherBodyIndex :type Integer) (bFromSweep :type Boolean) (SweepResult :type Hit%20Result%20Structure%20%28by%20ref%29))
  ;[1 1 1] open door if close enough
  (bind _asthird_person_character (Utilities|Casting|CastToThirdPersonCharacter OtherActor))
  (Input|EnableInput (Game|GetPlayerController 0) 0)
  (Utilities|FlowControl|Gate false) ; enters at Open
)

(event OnComponentEndOverlap(Box)
  (params (OverlappedComponent :type Primitive%20Component%20Object%20Reference) (OtherActor :type Actor%20Object%20Reference) (OtherComp :type Primitive%20Component%20Object%20Reference) (OtherBodyIndex :type Integer))
  ;[1 1 1] open door if close enough
  (Utilities|Casting|CastToThirdPersonCharacter OtherActor)
  (Input|DisableInput (Game|GetPlayerController 0) 0)
  (Utilities|FlowControl|Gate false) ; enters at Close
)

(event Input|ActionEvents|InputActioninteract
  (params (Key :type Key%20Structure :default "None"))
  ;[1 1 1] open door if close enough
  (:Pressed
    (if (Variables|/Game/ThirdPersonBP/Blueprints/ThirdPersonCharacter.ThirdPersonCharacter_C|Gethas_key? (stale OnComponentBeginOverlap(Box) _asthird_person_character))
      (Utilities|FlowControl|Gate false
        (:Exit
          ;[1 1 1] open/close door
          (Utilities|FlowControl|FlipFlop
            (:A
              (bind _door_track (Timeline|Open/close Play)
                (:Update
                  (Transformation|SetRelativeRotation (Variables|Default|GetDoor) (Math|Rotator|MakeRotator 0.0 0.0 (Math|Float|Lerp (Variables|Default|Getclosed_angle) (Variables|Default|Getopen_anlge) _door_track)) false false))))
            (:B
              (Timeline|Open/close Reverse)))))
      (else
        (Audio|PlaySoundatLocation "/Game/StarterContent/Audio/Collapse01.Collapse01" (Transformation|GetActorLocation) "0, 0, 0" 1.0 1.0 0.0 0 0 0 0)))))

(fn ConstructionScript)