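; Keypad door actor that swings open and closed, with a PIN check meant for a keypad widget.
; OpenDoor alternates between playing and reversing a timeline that lerps the door's yaw.
; AddToPin compares input to Pin; a match sets Unlocked, removes the widget and restores game-only input.
; The widget creation and toggle logic is disconnected, and OpenDoor does not check Unlocked.
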(event Custom|OpenDoor
  (Utilities|FlowControl|FlipFlop
    (:A
      (bind _dooranimation (Timeline|Open%20Door%20Timeline PlayFromStart)
        (:Update
          (Transformation|SetRelativeRotation (Variables|Default|GetDoor) (Math|Rotator|MakeRotator 0.0 0.0 (Math|Float|Lerp 0.0 1.2e+02 _dooranimation)) false false))))
    (:B
      (Timeline|Open%20Door%20Timeline Reverse))))

(fn ConstructionScript)

(fn AddtoPin
  (params (input :type String))
  (bind _returnvalue (Game|GetPlayerController 0))
  (if (Utilities|Enum|Equal(Enum) input (Variables|Default|Getpin))
    (Variables|Default|Setunlocked true)
    (Widget|RemovefromParent (Variables|Default|GetPin%20widget%20REF))
    (Input|SetInputModeGameOnly _returnvalue false)
    (Variables|/Script/Engine.PlayerController|SetbShowMouseCursor _returnvalue false)))